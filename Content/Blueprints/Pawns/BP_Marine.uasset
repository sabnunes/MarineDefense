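; Player-controlled marine for a twin-stick style shooter, with movement, yaw-only aiming, rifle fire, health, death and a kill count.
; Tick aims via control rotation from thumbstick angle or interpolated mouse velocity, both deadzone-filtered, switching on the last key's device.
; Holding fire runs a looping timer of muzzle line traces that apply damage and impact effects, with looped audio and muzzle flash.
; BeginPlay creates the HUD; damage reaching zero health sets Dead and stops firing.
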(event EventTick
  (params (DeltaSeconds :type Float%20%28single-precision%29))
  (CallFunction|UpdatePlayerAim))

(event EventBeginPlay
  (bind _returnvalue (UserInterface|CreateWidget "/Game/UI/W_PlayerHUD.W_PlayerHUD_C" 0 self))
  (UserInterface|Viewport|AddtoViewport _returnvalue 0))

(event Game|Damage|EventAnyDamage
  (params (Damage :type Float%20%28single-precision%29) (DamageType :type Damage%20Type%20Object%20Reference) (InstigatedBy :type Controller%20Object%20Reference) (DamageCauser :type Actor%20Object%20Reference))
  (if (CallFunction|IsAlive)
    (bind _health (CallFunction|DecreaseHealth Damage))
    (if (== _health 0.0)
      (Variables|Default|SetDead true)
      (CallFunction|EndFireWeapon))))

(event Input|ActionEvents|InputActionFireWeapon
  (params (Key :type Key%20Structure :default "None"))
  (:Pressed
    (CallFunction|StartFireWeapon))
  (:Released
    (CallFunction|EndFireWeapon)))

(event Input|AxisEvents|InputAxisMoveFrontBack
  (params (AxisValue :type Float%20%28single-precision%29))
  (if (CallFunction|IsAlive)
    (Pawn|Input|AddMovementInput (Math|Vector|MakeVector AxisValue (stale Input|AxisEvents|InputAxisMoveLeftRight AxisValue) 0.0) 1.0 false)))

(event Input|AxisEvents|InputAxisMoveLeftRight
  (params (AxisValue :type Float%20%28single-precision%29))
  (if (CallFunction|IsAlive)
    (Pawn|Input|AddMovementInput (Math|Vector|MakeVector (stale Input|AxisEvents|InputAxisMoveFrontBack AxisValue) AxisValue 0.0) 1.0 false)))

(event Input|KeyboardEvents|AnyKey
  (params (Key :type Key%20Structure :default "None"))
  (:Pressed
    (Variables|Default|SetGamepadActive (Class|KismetInputLibrary|KeyIsGamepadKey Key))))

(fn ConstructionScript)

(fn UpdatePlayerAim
  (if (and (CallFunction|IsAlive) (Variables|Default|GetGamepadActive))
    (ThumbstickInput|UpdateThumbstickAim)
    (else
      (MouseInput|UpdateMouseAim))))

(fn IsThumbstickAboveDeadzone
  (return (> (Math|Vector2D|Vector2DLength (Math|Vector2D|MakeVector2D (Input|AxisValues|GetThumbstickAimUp) (Input|AxisValues|GetThumbstickAimRight))) (Variables|ThumbstickInput|GetThumbstickDeadzone))))

(fn GetMouseVelocity
  (bind _returnvalue (Game|GetPlayerController 0))
  (bind (_deltax _deltay) (Class|PlayerController|GetInputMouseDelta _returnvalue))
  (return (/ (Math|Vector2D|MakeVector2D _deltax _deltay) (Utilities|Time|GetWorldDeltaSeconds))))

(fn IsMouseAboveDeadzone
  (return (> (Math|Vector2D|Vector2DLength (MouseInput|GetMouseVelocity)) (Variables|MouseInput|GetMouseDeadzone))))

(fn UpdateMouseAim
  (if (MouseInput|IsMouseAboveDeadzone)
    (Pawn|SetControlRotation (Game|GetPlayerController 0) (MouseInput|GetMouseAimDirection))))

(fn GetMouseAimDirection
  (bind _returnvalue (MouseInput|GetMouseVelocity))
  (return (Math|Interpolation|RInterpTo (Pawn|GetControlRotation (Game|GetPlayerController 0) :!class /Script/Engine.Controller) (Math|Rotator|MakeRotator 0.0 0.0 (Class|KismetMathLibrary|DegAtan2 (.x _returnvalue) (.y _returnvalue))) (Utilities|Time|GetWorldDeltaSeconds) (Variables|MouseInput|GetMouseInterpolateSpeed))))

(fn UpdateThumbstickAim
  (if (ThumbstickInput|IsThumbstickAboveDeadzone)
    (Pawn|SetControlRotation (Game|GetPlayerController 0) (Math|Rotator|MakeRotator 0.0 0.0 (Class|KismetMathLibrary|DegAtan2 (Input|AxisValues|GetThumbstickAimRight) (Input|AxisValues|GetThumbstickAimUp))))))

(fn StartFireWeapon
  (if (CallFunction|IsAlive)
    (Components|Activation|Activate (Variables|Default|GetP_Rifle_MuzzleFlash) false)
    (bind _returnvalue (Audio|SpawnSound2D "/Game/Sounds/Weapon_AssaultRifle/Stereo/RifleFireLoop_Cue.RifleFireLoop_Cue" 1.0 1.0 0.0 0))
    (Variables|Default|SetWeaponFireSound _returnvalue)
    (CallFunction|WeaponTrace)
    (Utilities|Time|SetTimerbyFunctionName 0 "WeaponTrace" (Variables|Default|GetWeaponFireRate) true)))

(fn EndFireWeapon
  (bind _weaponfiresound (Variables|Default|GetWeaponFireSound))
  (Components|Activation|Deactivate (Variables|Default|GetP_Rifle_MuzzleFlash))
  (Utilities|IsValid _weaponfiresound
    (:Is%20Valid
      (Audio|Components|Audio|Stop _weaponfiresound)
      (Utilities|Time|ClearTimerbyFunctionName 0 "WeaponTrace")
      (if (CallFunction|IsAlive)
        (Audio|SpawnSound2D "/Game/Sounds/Weapon_AssaultRifle/Stereo/RifleFireEnd_Cue.RifleFireEnd_Cue" 1.0 1.0 0.0 0)))))

(fn DecreaseHealth
  (params (DamageAmount :type Float%20%28double-precision%29))
  (bind _output_get (Variables|PlayerProperties|SetHealth (Math|Float|Clamp(Float) (- (Variables|PlayerProperties|GetHealth) DamageAmount) 0.0 1e+02)))
  (return _output_get))

(fn IsAlive
  (return (not (Variables|Default|GetDead))))

(fn WeaponTrace
  (bind _outhit (Collision|LineTraceByChannel (CallFunction|GetWeaponTraceStartLocation) (CallFunction|GetWeaponTraceEndLocation) "TraceTypeQuery1" false 0 "None"))
  (if (.bBlockingHit (Collision|BreakHitResult _outhit))
    (Game|Damage|ApplyDamage (.HitActor (Collision|BreakHitResult _outhit)) (Variables|Default|GetDamagePerShot) 0 0)
    (CallFunction|SpawnHitImpact (.Location (Collision|BreakHitResult _outhit)))))

(fn GetWeaponTraceStartLocation
  (return (Transformation|GetSocketLocation (Variables|Default|GetSK_Rifle) "MuzzleFlash")))

(fn GetWeaponTraceEndLocation
  (return (+ (* (Math|Vector|GetForwardVector (Pawn|GetControlRotation :!class /Script/Engine.Pawn)) (Variables|Default|GetWeaponRange)) (CallFunction|GetWeaponTraceStartLocation))))

(fn IncreaseKills
  (Math|Integer|IncrementInt (Variables|PlayerProperties|GetKills)))

(fn SpawnHitImpact
  (params (HitLocation :type Vector))
  (Effects|SpawnEmitteratLocation "/Game/Effects/Weapons/Impacts/P_AssaultRifle_IH.P_AssaultRifle_IH" HitLocation))

(fn AddHealth
  (params (HealthPickUp :type Float%20%28double-precision%29))
  (Variables|PlayerProperties|SetHealth (Math|Float|Clamp(Float) (+ (Variables|PlayerProperties|GetHealth) HealthPickUp) 0.0 1e+02)))

(fn IsHealthFull
  (return (== (Variables|PlayerProperties|GetHealth) 1e+02)))